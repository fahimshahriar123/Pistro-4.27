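; BP_Goblin is a flipbook enemy that chases the player and fails the mission on contact.
; While ChangeLocation is true, Tick moves it toward the player with constant-speed interpolation and no sweep, switching between walk and idle flipbooks.
; Sphere overlap with BP_ManChar disables input, shows the failure widget and loads Level_5 after a delay.
; Bullet overlaps drain Health, raise speed at set thresholds, and on death remove a BP_BlockingCube.
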(event `self.ReceiveBeginPlay`)

(event `self.ReceiveTick`
  (params (DeltaSeconds :type "Float (single-precision)"))
  (if (`self.Change Location`)
    (`self.K2_SetActorLocation` (`KismetMathLibrary.VInterpTo_Constant` (`SceneComponent.K2_GetComponentLocation` (`self.CapsuleComponent`)) (`SceneComponent.K2_GetComponentLocation` (`Character.CapsuleComponent` (`GameplayStatics.GetPlayerCharacter` 0))) DeltaSeconds (`self.Interp Speed`)))
    (`PaperFlipbookComponent.SetFlipbook` (`self.Sprite`) "/Game/Assets/Textures/Flipbooks/Goblin/FL_GobWalk.FL_GobWalk")
    (else
      (`PaperFlipbookComponent.SetFlipbook` (`self.Sprite`) "/Game/Assets/Textures/Flipbooks/Goblin/FL_GobIdle.FL_GobIdle"))))

(event `self.Sphere.OnComponentBeginOverlap`
  (params (OverlappedComponent :type "PrimitiveComponent Object Reference") (OtherActor :type "Actor Object Reference") (OtherComp :type "PrimitiveComponent Object Reference") (OtherBodyIndex :type Integer) (bFromSweep :type Boolean) (SweepResult :type "HitResult Structure (by ref)"))
  (`|ExecutionSequence`
    (:`then_0`
      (cast `/Game/Assets/Blueprints/BP_ManChar` OtherActor)
      (`self.DisableInput` (`GameplayStatics.GetPlayerCharacter` 0) null)
      (set `self.Change Location` false)
      (set `self.Mission Failed` true)
      (bind _returnvalue (`|CreateWidget` "/Game/Widgets/BP_MissionFailed2.BP_MissionFailed2_C"))
      (`UserWidget.AddToViewport` _returnvalue 0)
      (`KismetSystemLibrary.Delay` 7.75)
      (`GameplayStatics.OpenLevel` "Level_5"))
    (:`then_1`
      (bind _asbp_bullet (cast `/Game/Assets/Blueprints/BP_Bullet` OtherActor))
      (`self.K2_DestroyActor` _asbp_bullet)
      (bind _output_get (set `self.Health` (- (`self.Health`) 50)))
      (if (== _output_get 500)
        (set `self.Interp Speed` 220.0)
        (elif (== _output_get 300)
          (set `self.Interp Speed` 250.0)))
      (if (<= _output_get 0)
        (`self.K2_DestroyActor`)
        (bind _outactors (`GameplayStatics.GetAllActorsOfClass` "/Game/Assets/Blueprints/BP_BlockingCube.BP_BlockingCube_C"))
        (`self.K2_DestroyActor` (`|GetArrayItem` _outactors))))))

(fn `UserConstructionScript`)