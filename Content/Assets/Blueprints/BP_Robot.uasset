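; BP_Robot is a 2D flipbook character that chases BP_ManChar pawns it spots through PawnSensing, using AIMoveTo.
; It also carries player-style MoveRight and Jump input handlers and sets its walk speed on BeginPlay.
; Tick picks idle, run, jump or land flipbooks from the Man set based on velocity and falling state.
; Tick also flips player controller 0's yaw, not its own controller's, from this character's horizontal velocity.
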(event `InputAxis|MoveRight`
  (params (AxisValue :type "Float (single-precision)"))
  ;[1 1 1] Controller
  (`self.AddMovementInput` (1.0 0.0 0.0) AxisValue))

(event `self.ReceiveBeginPlay`
  (set `CharacterMovementComponent.MaxWalkSpeed` 300.0 (`self.CharacterMovement`)))

(event `InputAction|Jump`
  (params (Key :type "Key Structure"))
  ;[1 1 1] Controller
  (:`Pressed`
    (`self.Jump`)))

(event `self.ReceiveTick`
  (params (DeltaSeconds :type "Float (single-precision)"))
  (bind _returnvalue_x (`KismetMathLibrary.BreakVector` (`self.GetVelocity`)))
  (bind _returnvalue (`GameplayStatics.GetPlayerController` 0))
  (bind (_returnvalue_x_2 _returnvalue_y _returnvalue_z) (`KismetMathLibrary.BreakVector` (`self.GetVelocity`)))
  (bind _sprite (`self.Sprite`))
  (`|ExecutionSequence`
    (:`then_0`
      ;[1 1 1] Play Animation
      (if (`NavMovementComponent.IsFalling` (`self.CharacterMovement`))
        (`PaperFlipbookComponent.SetFlipbook` (`self.Sprite`) (select `bool` (<= _returnvalue_z 0.0) :`false` "/Game/Assets/Textures/Flipbooks/Man/FL_ManJump.FL_ManJump" :`true` "/Game/Assets/Textures/Flipbooks/Man/FL_ManLand.FL_ManLand" :!type "PaperFlipbook Object Reference"))
        (elif (!= (`KismetMathLibrary.VSize` (`self.GetVelocity`)) 0.0)
          (`PaperFlipbookComponent.SetFlipbook` _sprite "/Game/Assets/Textures/Flipbooks/Man/FL_ManRun.FL_ManRun")
          (else
            (`PaperFlipbookComponent.SetFlipbook` _sprite "/Game/Assets/Textures/Flipbooks/Man/FL_ManIdle.FL_ManIdle")))))
    (:`then_1`
      ;[1 1 1] Character Rotation
      (`/Engine/EditorBlueprintResources/StandardMacros.CompareFloat` _returnvalue_x
        (:`>`
          (`Controller.SetControlRotation` _returnvalue (`KismetMathLibrary.MakeRotator` 0.0)))
        (:`<`
          (`Controller.SetControlRotation` _returnvalue (`KismetMathLibrary.MakeRotator` 0.0 0.0 180.0)))))))

(event `self.PawnSensing.OnSeePawn`
  (params (Pawn :type "Pawn Object Reference"))
  (bind _asbp_man_char (cast `/Game/Assets/Blueprints/BP_ManChar` Pawn))
  (`|AIMoveTo` self (0.0 0.0 0.0) _asbp_man_char))

(fn `UserConstructionScript`)