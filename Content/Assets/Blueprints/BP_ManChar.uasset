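; BP_ManChar is a side-view Paper2D player character that runs along world X, jumps and shoots.
; Tick picks the idle, run, jump or land flipbook from falling state and velocity.
; It also flips facing by setting control rotation yaw from the sign of X velocity.
; Fire, gated by CanFire, spawns a scaled-down BP_Bullet with the actor's location and rotation and plays a laser sound.
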(event `InputAxis|MoveRight`
  (params (AxisValue :type "Float (single-precision)"))
  ;[1 1 1] Controller
  (`self.AddMovementInput` (1.0 0.0 0.0) AxisValue))

(event `self.ReceiveBeginPlay`
  (set `CharacterMovementComponent.MaxWalkSpeed` 300.0 (`self.CharacterMovement`)))

(event `InputAction|Jump`
  (params (Key :type "Key Structure"))
  ;[1 1 1] Controller
  (:`Pressed`
    (`self.Jump`)))

(event `self.ReceiveTick`
  (params (DeltaSeconds :type "Float (single-precision)"))
  (bind _returnvalue_x (`KismetMathLibrary.BreakVector` (`self.GetVelocity`)))
  (bind _returnvalue (`GameplayStatics.GetPlayerController` 0))
  (bind (_returnvalue_x_2 _returnvalue_y _returnvalue_z) (`KismetMathLibrary.BreakVector` (`self.GetVelocity`)))
  (bind _sprite (`self.Sprite`))
  (`|ExecutionSequence`
    (:`then_0`
      ;[1 1 1] Play Animation
      (if (`NavMovementComponent.IsFalling` (`self.CharacterMovement`))
        (`PaperFlipbookComponent.SetFlipbook` (`self.Sprite`) (select `bool` (<= _returnvalue_z 0.0) :`false` "/Game/Assets/Textures/Flipbooks/Man/FL_ManJump.FL_ManJump" :`true` "/Game/Assets/Textures/Flipbooks/Man/FL_ManLand.FL_ManLand" :!type "PaperFlipbook Object Reference"))
        (elif (!= (`KismetMathLibrary.VSize` (`self.GetVelocity`)) 0.0)
          (`PaperFlipbookComponent.SetFlipbook` _sprite "/Game/Assets/Textures/Flipbooks/Man/FL_ManRun.FL_ManRun")
          (else
            (`PaperFlipbookComponent.SetFlipbook` _sprite "/Game/Assets/Textures/Flipbooks/Man/FL_ManIdle.FL_ManIdle")))))
    (:`then_1`
      ;[1 1 1] Character Rotation
      (`/Engine/EditorBlueprintResources/StandardMacros.CompareFloat` _returnvalue_x
        (:`>`
          (`Controller.SetControlRotation` _returnvalue (`KismetMathLibrary.MakeRotator` 0.0)))
        (:`<`
          (`Controller.SetControlRotation` _returnvalue (`KismetMathLibrary.MakeRotator` 0.0 0.0 180.0)))))))

(event `InputAction|Fire`
  (params (Key :type "Key Structure"))
  (bind _returnvalue (`self.K2_GetActorLocation`))
  (:`Pressed`
    (if (`self.Can Fire`)
      (`|SpawnActorFromClass` "/Game/Assets/Blueprints/BP_Bullet.BP_Bullet_C" (`KismetMathLibrary.MakeTransform` _returnvalue (`self.K2_GetActorRotation`) (0.2 0.2 0.2)) "Undefined" "OverrideRootScale" null null)
      (`GameplayStatics.PlaySoundAtLocation` "/Game/Assets/Sounds/Laser_Gun_Sound_Effect.Laser_Gun_Sound_Effect" _returnvalue (struct) 1.0 1.0 0.0 null null null))))

(fn `UserConstructionScript`)